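; Player character for a Bomberman-style Paper2D game, moved along world X and Z by input axes, with the camera detached at BeginPlay.
; Each tick SetAnimation stores the last move direction and picks a walk or idle flipbook from it and velocity.
; Left reuses the right-facing flipbooks by rotating the sprite 180 degrees.
; Capsule overlap with fire or an enemy calls PlayerHasDied.
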(event OnComponentBeginOverlap(CapsuleComponent)
  (params (OverlappedComponent :type Primitive%20Component%20Object%20Reference) (OtherActor :type Actor%20Object%20Reference) (OtherComp :type Primitive%20Component%20Object%20Reference) (OtherBodyIndex :type Integer) (bFromSweep :type Boolean) (SweepResult :type Hit%20Result%20Structure%20%28by%20ref%29))
  (Utilities|FlowControl|Sequence
    (:then_0
      (Utilities|Casting|CastToFire_BP OtherActor))
    (:then_1
      (Utilities|Casting|CastToEnemyPaper_BP OtherActor)))
  (Default|CallPlayerHasDied))

(event EventBeginPlay
  (Transformation|DetachFromComponent (Variables|Default|GetCamera) "KeepRelative" "KeepRelative" "KeepRelative" true))

(event EventTick
  (params (DeltaSeconds :type Float%20%28single-precision%29))
  (CallFunction|SetAnimation))

(event Input|AxisEvents|InputAxisMoveForward
  (params (AxisValue :type Float%20%28single-precision%29))
  (Pawn|Input|AddMovementInput "0.000000,0.000000,1.000000" AxisValue false))

(event Input|AxisEvents|InputAxisMoveRight
  (params (AxisValue :type Float%20%28single-precision%29))
  (Pawn|Input|AddMovementInput "1.000000,0.000000, 0" AxisValue false))

(fn ConstructionScript)

(fn SetAnimation
  (bind _sprite (Variables|Default|GetSprite))
  (if (or (!= (Input|AxisValues|GetMoveForward) 0.0) (!= (Input|AxisValues|GetMoveRight) 0.0))
    (Variables|Default|SetLastMoveDirection (select (< (Input|AxisValues|GetMoveRight) 0.0) "NewEnumerator2" (select (> (Input|AxisValues|GetMoveRight) 0.0) "NewEnumerator3" (select (< (Input|AxisValues|GetMoveForward) 0.0) "NewEnumerator0" (select (> (Input|AxisValues|GetMoveForward) 0.0) "NewEnumerator1" "NewEnumerator0"))))))
  (Sprite|SetFlipbook (Variables|Default|GetSprite) (select (> (Math|Vector|VectorLength (Transformation|GetVelocity)) 0.0) (Utilities|Select :Index (Variables|Default|GetLastMoveDirection) :NewEnumerator0 "/Game/Bomberman/Sprites/PlayerWalkDown/PlayerWalkDown.PlayerWalkDown" :NewEnumerator1 "/Game/Bomberman/Sprites/PlayerWalkUp/PlayerWalkUp.PlayerWalkUp" :NewEnumerator2 "/Game/Bomberman/Sprites/PlayerWalkRight/PlayerWalkRight.PlayerWalkRight" :NewEnumerator3 "/Game/Bomberman/Sprites/PlayerWalkRight/PlayerWalkRight.PlayerWalkRight") (Utilities|Select :Index (Variables|Default|GetLastMoveDirection) :NewEnumerator0 "/Game/Bomberman/Sprites/PlayerIdle/PlayerIdleDown.PlayerIdleDown" :NewEnumerator1 "/Game/Bomberman/Sprites/PlayerIdle/PlayerIdleUp.PlayerIdleUp" :NewEnumerator2 "/Game/Bomberman/Sprites/PlayerIdle/PlayerIdleRight.PlayerIdleRight" :NewEnumerator3 "/Game/Bomberman/Sprites/PlayerIdle/PlayerIdleRight.PlayerIdleRight")))
  (if (Utilities|Enum|Equal(Enum) (Variables|Default|GetLastMoveDirection) "NewEnumerator2")
    (Transformation|SetRelativeRotation _sprite "0,180.000000, 0" false false)
    (else
      (Transformation|SetRelativeRotation _sprite "0, 0, 0" false false))))