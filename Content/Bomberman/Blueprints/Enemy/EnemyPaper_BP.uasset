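; Bomberman enemy that patrols back and forth along one axis and dies when it overlaps fire.
; On BeginPlay, MovementDirection selects local X or Z as the axis for the ProjectileMovement velocity.
; Box hits and overlaps with blocks, bombs or BombermanGameplay reverse it by negating the Box's physics linear velocity and passing that back as local-space velocity.
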(event OnComponentHit(Box)
  (params (HitComponent :type Primitive%20Component%20Object%20Reference) (OtherActor :type Actor%20Object%20Reference) (OtherComp :type Primitive%20Component%20Object%20Reference) (NormalImpulse :type Vector :default "0, 0, 0") (Hit :type Hit%20Result%20Structure%20%28by%20ref%29))
  (CallFunction|InvertDirection))

(event EventBeginPlay
  (CallFunction|SetInitialMovement))

(event Collision|EventActorBeginOverlap
  (params (OtherActor :type Actor%20Object%20Reference))
  (Utilities|FlowControl|Sequence
    (:then_0
      (Utilities|Casting|CastToBlock_BP OtherActor)
      (CallFunction|InvertDirection :!label _label))
    (:then_1
      (Utilities|Casting|CastToBombermanGameplay OtherActor)
      (goto _label))
    (:then_2
      (Utilities|Casting|CastToBomb_BP OtherActor)
      (goto _label))
    (:then_3
      (Utilities|Casting|CastToFire_BP OtherActor)
      (Actor|DestroyActor))))

(fn ConstructionScript)

(fn SetInitialMovement
  (bind _velocity (Variables|Default|GetVelocity))
  (if (Utilities|Enum|Equal(Enum) (Variables|Default|GetMovementDirection) "NewEnumerator0")
    (LocalVariables|SetVelocityX _velocity)
    (else
      (LocalVariables|SetVelocityZ _velocity)))
  (Game|Components|ProjectileMovement|SetVelocityinLocalSpace (Variables|Default|GetProjectileMovement) (Math|Vector|MakeVector (LocalVariables|GetVelocityX) 0.0 (LocalVariables|GetVelocityZ))))

(fn InvertDirection
  (bind _returnvalue (Physics|GetPhysicsLinearVelocity (Variables|Default|GetBox) "None"))
  (Game|Components|ProjectileMovement|SetVelocityinLocalSpace (Variables|Default|GetProjectileMovement) (Math|Vector|MakeVector (* (.x _returnvalue) -1.0) 0.0 (* (.z _returnvalue) -1.0))))