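; Bomberman enemy actor that moves in a straight line along one axis and reacts when it overlaps the player.
; On BeginPlay it sets its ProjectileMovement velocity on local X or Z, chosen by the MovementDirection enum.
; InvertDirection negates the current X and Z velocity, but nothing in this graph calls it.
; Player overlap calls HasOverlapedActor on the player and prints a debug string.
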(event Collision|EventActorBeginOverlap
  (params (OtherActor :type Actor%20Object%20Reference))
  (Utilities|Casting|CastToPlayer OtherActor)
  (Default|CallHasOverlapedActor)
  (Development|PrintString "Overlap player"))

(event EventBeginPlay
  (CallFunction|SetInitialMovement))

(fn ConstructionScript)

(fn SetInitialMovement
  (bind _velocity (Variables|Default|GetVelocity))
  (if (Utilities|Enum|Equal(Enum) (Variables|Default|GetMovementDirection) "NewEnumerator0")
    (LocalVariables|SetVelocityX _velocity)
    (else
      (LocalVariables|SetVelocityZ _velocity)))
  (Game|Components|ProjectileMovement|SetVelocityinLocalSpace (Variables|Default|GetProjectileMovement) (Math|Vector|MakeVector (LocalVariables|GetVelocityX) 0.0 (LocalVariables|GetVelocityZ))))

(fn InvertDirection
  (bind _returnvalue (Transformation|GetVelocity))
  (Game|Components|ProjectileMovement|SetVelocityinLocalSpace (Variables|Default|GetProjectileMovement) (Math|Vector|MakeVector (* (.x _returnvalue) -1.0) 0.0 (* (.z _returnvalue) -1.0))))