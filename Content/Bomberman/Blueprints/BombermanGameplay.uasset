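; Bomberman gameplay controller that runs a tilemap level, from intro widget and music to restart after player death.
; BeginPlay spawns destructible blocks from a coordinate array, keeping actor references in a parallel array.
; PlaceBomb input spawns a bomb snapped to the player's tile center.
; On explosion, it scans four directions up to ExplosionLength, stopping at blocks or boundary-layer tiles, then destroys hit blocks and spawns fire.
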(event Custom|CustomEvent_0
  (CallFunction|HandleBombExploded (stale Input|ActionEvents|InputActionPlaceBomb _tile_center_transform)))

(event Custom|PlayerHasDied_Event_0
  (Utilities|Time|SetTimerbyEvent (delegate Custom|CustomEvent_1) 0.5))

(event Custom|CustomEvent_1
  (Default|CallRestart))

(event Custom|CustomEvent_2
  (Viewport|RemoveAllWidgets)
  (bind _returnvalue (Audio|CreateSound2D "/Game/Bomberman/Audios/theme_bomberman.theme_bomberman" 0.5 1.0 0.1 0))
  (bind _output_get (Variables|Default|SetThemeSound _returnvalue))
  (Audio|Components|Audio|Play _output_get 0.0))

(event EventBeginPlay
  (CallFunction|SavePlayerRef)
  (Input|EnableInput (Game|GetPlayerController 0))
  (Class|PaperTileMapComponent|MakeTileMapEditable (Variables|Default|GetTilemap))
  (CallFunction|SpawnBlocks)
  (EventDispatchers|AssignPlayerHasDied (Variables|Default|GetBombermanPlayerRef) (delegate Custom|PlayerHasDied_Event_0))
  (bind _returnvalue (Audio|CreateSound2D "/Game/Bomberman/Audios/intro.intro" 1.0 1.0 0.1 0))
  (Audio|Components|Audio|Play _returnvalue 0.0)
  (bind _returnvalue_2 (UserInterface|CreateWidget "/Game/Bomberman/Blueprints/Introduction.Introduction_C"))
  (UserInterface|Viewport|AddtoViewport _returnvalue_2 0)
  (Utilities|Time|SetTimerbyEvent (delegate Custom|CustomEvent_2) 1.7))

(event Input|ActionEvents|InputActionPlaceBomb
  (params (Key :type Key%20Structure :default "None"))
  (:Pressed
    (bind _tile_center_transform (CallFunction|GetTileCenterTransform (Transformation|GetWorldTransform (Components|GetChildComponent (Variables|Default|GetBombermanPlayer) 0))))
    (bind _returnvalue (Game|SpawnActorfromClass "/Game/Bomberman/Blueprints/Bomb_BP.Bomb_BP_C" (Math|Transform|MakeTransform (Math|Vector|MakeVector (.x (.Location (Math|Transform|BreakTransform _tile_center_transform))) 1e+01 (.z (.Location (Math|Transform|BreakTransform _tile_center_transform)))) (.Rotation (Math|Transform|BreakTransform _tile_center_transform)) (.Scale (Math|Transform|BreakTransform _tile_center_transform))) "Undefined" 0 0))
    (EventDispatchers|BindEventtoBombExploded _returnvalue (delegate Custom|CustomEvent_0))))

(fn ConstructionScript)

(fn EnablePlayerInput
  (Pawn|Possess (Game|GetPlayerController 0) (Variables|Default|GetBombermanPlayerRef))
  (Audio|Components|Audio|SetVolumeMultiplier (Variables|Default|GetThemeSound) 0.5 :!class /Script/Engine.AudioComponent))

(fn DIsablePlayerInput
  (Audio|Components|Audio|SetVolumeMultiplier (Variables|Default|GetThemeSound) 0.05 :!class /Script/Engine.AudioComponent))

(fn SavePlayerRef
  (bind _asbomberman_player (Utilities|Casting|CastToBombermanPlayer (Variables|/Script/Engine.ChildActorComponent|GetChildActor (Variables|Default|GetBombermanPlayer))))
  (Variables|Default|SetBombermanPlayerRef _asbomberman_player))

(fn GetTileCenterTransform
  (params (Transform%20Reference :type Transform))
  (bind (_x _y) (CallFunction|GetTileIndexbyLocation (.location Transform%20Reference)))
  (return (Math|Transform|MakeTransform (Class|PaperTileMapComponent|GetTileCenterPosition (Variables|Default|GetTilemap) _x _y 0 true) (.rotation Transform%20Reference) (.scale Transform%20Reference))))

(fn GetTileIndexbyLocation
  (params (Reference%20Location :type Vector))
  (return (Math|Float|Truncate (|(pos/size) (.x Reference%20Location) (Variables|Default|GetTile%20Width))) (Math|Float|Truncate (|(pos/size) (Math|Float|Absolute(Float) (.z Reference%20Location)) (Variables|Default|GetTile%20Height)))))

(fn HandleBombExploded
  (params (NewParam :type Transform))
  (bind (_x _y) (CallFunction|GetTileIndexbyLocation (.location NewParam)))
  (LocalVariables|SetX _x)
  (LocalVariables|SetY _y)
  (Utilities|FlowControl|Sequence
    (:then_0
      ;[1 1 1] Top tiles
      (bind _index (Utilities|FlowControl|ForLoopwithBreak 1 (Variables|Default|GetExplosion%20Length) :!label _label)
        (:LoopBody
          (bind _doesexist (CallFunction|FindinBlocks (Utilities|Struct|MakeCoordinate (LocalVariables|GetX) (- (LocalVariables|GetY) _index))))
          (if _doesexist
            (Utilities|Array|Add (LocalVariables|GetToSetFire) (Utilities|Struct|MakeCoordinate (LocalVariables|GetX) (- (LocalVariables|GetY) _index)))
            (Utilities|Array|Add (LocalVariables|GetToDestroy) (Utilities|Struct|MakeCoordinate (LocalVariables|GetX) (- (LocalVariables|GetY) _index)))
            (goto _label Break)
            (else
              (Utilities|IsValid (.tileset (Class|PaperTileMapComponent|GetTile (Variables|Default|GetTilemap) (.X (Utilities|Struct|BreakCoordinate (Utilities|Struct|MakeCoordinate (LocalVariables|GetX) (- (LocalVariables|GetY) _index)))) (.Y (Utilities|Struct|BreakCoordinate (Utilities|Struct|MakeCoordinate (LocalVariables|GetX) (- (LocalVariables|GetY) _index)))) (Variables|Default|GetBoundary%20Layer)))
                (:Is%20Valid
                  (goto _label Break))
                (:Is%20Not%20Valid
                  (Utilities|Array|Add (LocalVariables|GetToSetFire) (Utilities|Struct|MakeCoordinate (LocalVariables|GetX) (- (LocalVariables|GetY) _index))))))))))
    (:then_1
      ;[1 1 1] Bottom tiles
      (bind _index_2 (Utilities|FlowControl|ForLoopwithBreak 1 (Variables|Default|GetExplosion%20Length) :!label _label_2)
        (:LoopBody
          (bind _doesexist_2 (CallFunction|FindinBlocks (Utilities|Struct|MakeCoordinate (LocalVariables|GetX) (+ (LocalVariables|GetY) _index_2))))
          (if _doesexist_2
            (Utilities|Array|Add (LocalVariables|GetToSetFire) (Utilities|Struct|MakeCoordinate (LocalVariables|GetX) (+ (LocalVariables|GetY) _index_2)))
            (Utilities|Array|Add (LocalVariables|GetToDestroy) (Utilities|Struct|MakeCoordinate (LocalVariables|GetX) (+ (LocalVariables|GetY) _index_2)))
            (goto _label_2 Break)
            (else
              (Utilities|IsValid (.tileset (Class|PaperTileMapComponent|GetTile (Variables|Default|GetTilemap) (.X (Utilities|Struct|BreakCoordinate (Utilities|Struct|MakeCoordinate (LocalVariables|GetX) (+ (LocalVariables|GetY) _index_2)))) (.Y (Utilities|Struct|BreakCoordinate (Utilities|Struct|MakeCoordinate (LocalVariables|GetX) (+ (LocalVariables|GetY) _index_2)))) (Variables|Default|GetBoundary%20Layer)))
                (:Is%20Valid
                  (goto _label_2 Break))
                (:Is%20Not%20Valid
                  (Utilities|Array|Add (LocalVariables|GetToSetFire) (Utilities|Struct|MakeCoordinate (LocalVariables|GetX) (+ (LocalVariables|GetY) _index_2))))))))))
    (:then_2
      ;[1 1 1] Left tiles
      (bind _index_3 (Utilities|FlowControl|ForLoopwithBreak 1 (Variables|Default|GetExplosion%20Length) :!label _label_3)
        (:LoopBody
          (bind _doesexist_3 (CallFunction|FindinBlocks (Utilities|Struct|MakeCoordinate (- (LocalVariables|GetX) _index_3) (LocalVariables|GetY))))
          (if _doesexist_3
            (Utilities|Array|Add (LocalVariables|GetToSetFire) (Utilities|Struct|MakeCoordinate (- (LocalVariables|GetX) _index_3) (LocalVariables|GetY)))
            (Utilities|Array|Add (LocalVariables|GetToDestroy) (Utilities|Struct|MakeCoordinate (- (LocalVariables|GetX) _index_3) (LocalVariables|GetY)))
            (goto _label_3 Break)
            (else
              (Utilities|IsValid (.tileset (Class|PaperTileMapComponent|GetTile (Variables|Default|GetTilemap) (.X (Utilities|Struct|BreakCoordinate (Utilities|Struct|MakeCoordinate (- (LocalVariables|GetX) _index_3) (LocalVariables|GetY)))) (.Y (Utilities|Struct|BreakCoordinate (Utilities|Struct|MakeCoordinate (- (LocalVariables|GetX) _index_3) (LocalVariables|GetY)))) (Variables|Default|GetBoundary%20Layer)))
                (:Is%20Valid
                  (goto _label_3 Break))
                (:Is%20Not%20Valid
                  (Utilities|Array|Add (LocalVariables|GetToSetFire) (Utilities|Struct|MakeCoordinate (- (LocalVariables|GetX) _index_3) (LocalVariables|GetY))))))))))
    (:then_3
      ;[1 1 1] Right tiles
      (bind _index_4 (Utilities|FlowControl|ForLoopwithBreak 1 (Variables|Default|GetExplosion%20Length) :!label _label_4)
        (:LoopBody
          (bind _doesexist_4 (CallFunction|FindinBlocks (Utilities|Struct|MakeCoordinate (+ (LocalVariables|GetX) _index_4) (LocalVariables|GetY))))
          (if _doesexist_4
            (Utilities|Array|Add (LocalVariables|GetToSetFire) (Utilities|Struct|MakeCoordinate (+ (LocalVariables|GetX) _index_4) (LocalVariables|GetY)))
            (Utilities|Array|Add (LocalVariables|GetToDestroy) (Utilities|Struct|MakeCoordinate (+ (LocalVariables|GetX) _index_4) (LocalVariables|GetY)))
            (goto _label_4 Break)
            (else
              (Utilities|IsValid (.tileset (Class|PaperTileMapComponent|GetTile (Variables|Default|GetTilemap) (.X (Utilities|Struct|BreakCoordinate (Utilities|Struct|MakeCoordinate (+ (LocalVariables|GetX) _index_4) (LocalVariables|GetY)))) (.Y (Utilities|Struct|BreakCoordinate (Utilities|Struct|MakeCoordinate (+ (LocalVariables|GetX) _index_4) (LocalVariables|GetY)))) (Variables|Default|GetBoundary%20Layer)))
                (:Is%20Valid
                  (goto _label_4 Break))
                (:Is%20Not%20Valid
                  (Utilities|Array|Add (LocalVariables|GetToSetFire) (Utilities|Struct|MakeCoordinate (+ (LocalVariables|GetX) _index_4) (LocalVariables|GetY))))))))))
    (:then_4
      ;[1 1 1] Center Tile
      (Utilities|Array|Add (LocalVariables|GetToSetFire) (Utilities|Struct|MakeCoordinate (LocalVariables|GetX) (LocalVariables|GetY))))
    (:then_5
      (for _array_element (LocalVariables|GetToDestroy)
        (if (Utilities|IsValid (Utilities|Array|Get(acopy) (Variables|Default|GetBlockRefs) (Utilities|Array|FindItem (Variables|Default|GetBlocks) (Utilities|Struct|MakeCoordinate (.x _array_element) (.y _array_element)))))
          (Actor|DestroyActor (Utilities|Array|Get(acopy) (Variables|Default|GetBlockRefs) (Utilities|Array|FindItem (Variables|Default|GetBlocks) (Utilities|Struct|MakeCoordinate (.x _array_element) (.y _array_element))))))))
    (:then_6
      (for _array_element_2 (LocalVariables|GetToSetFire)
        (Game|SpawnActorfromClass "/Game/Bomberman/Blueprints/Fire_BP.Fire_BP_C" (Math|Transform|MakeTransform (Math|Vector|MakeVector (.x (Class|PaperTileMapComponent|GetTileCenterPosition (Variables|Default|GetTilemap) (.x _array_element_2) (.y _array_element_2) (Variables|Default|GetGround%20Layer) true)) 5.0 (.z (Class|PaperTileMapComponent|GetTileCenterPosition (Variables|Default|GetTilemap) (.x _array_element_2) (.y _array_element_2) (Variables|Default|GetGround%20Layer) true))) "0, 0, 0" "1,1,1") "AlwaysSpawn" 0 0)))))

(fn SpawnBlocks
  (for _array_element (Variables|Default|GetBlocks)
    (bind _returnvalue (Game|SpawnActorfromClass "/Game/Bomberman/Blueprints/Block_BP.Block_BP_C" (Math|Transform|MakeTransform (Math|Vector|MakeVector (.x (Class|PaperTileMapComponent|GetTileCenterPosition (Variables|Default|GetTilemap) (.x _array_element) (.y _array_element) 0 true)) 1e+01 (.z (Class|PaperTileMapComponent|GetTileCenterPosition (Variables|Default|GetTilemap) (.x _array_element) (.y _array_element) 0 true))) "0, 0, 0" "1,1,1") "AlwaysSpawn" 0 0))
    (Utilities|Array|Add (Variables|Default|GetBlockRefs) _returnvalue)))

(fn FindinBlocks
  (params (Coordinate :type Coordinate%20Structure))
  (return (> (Utilities|Array|FindItem (Variables|Default|GetBlocks) (Utilities|Struct|MakeCoordinate (.x Coordinate) (.y Coordinate))) -1)))